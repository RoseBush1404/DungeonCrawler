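; Inventory manager for a dungeon crawler character, handling item pickup, drop, equip and unequip, plus spawning of starting gear.
; Items move between a size-capped Inventory and type-indexed weapon, armour and trinket slots according to ItemState, with equipped items attaching to mesh sockets.
; Drops teleport to random navigable points near the owner, and unequipping falls back to dropping when full.
; Actions check owner status, refresh the GUI and report pickups and drops.
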(fn ConstructionScript)

(fn PickUpItem
  (params (ItemToPickUp :type Inventory%20Item%20Object%20Reference))
  (bind _gamegui (Variables|References|GetGameGUI))
  (bind _statusfree (Default|CheckStatus (Variables|References|GetDCOwner) (Utilities|Struct|MakeStatus false false false false false false true)))
  (if _statusfree
    (if (< (Utilities|Array|Length (Variables|Default|GetInventory)) (Variables|Default|GetInventorySize))
      (Utilities|IsValid ItemToPickUp
        (:Is%20Valid
          (switch Utilities|FlowControl|Switch|SwitchonItemStates (Variables|/Game/DungeonCrawlerContent/Blueprints/Inventory/InventoryItem.InventoryItem_C|GetItemState ItemToPickUp)
            (:NewEnumerator0
              _)
            (:NewEnumerator2
              _))
          (Default|ChangeItemState ItemToPickUp "NewEnumerator1")
          (Utilities|Array|Add (Variables|Default|GetInventory) ItemToPickUp)
          (Transformation|SetActorLocation ItemToPickUp "0.000000, 0, 0" false false)
          (Variables|/Game/DungeonCrawlerContent/Blueprints/Inventory/InventoryItem.InventoryItem_C|SetDCOwner ItemToPickUp (Variables|References|GetDCOwner))
          (Class|MessageInterface|SendMessage(Message) (Game|GetGameInstance) (Utilities|String|Append (Utilities|String|ToString(Name) (Variables|/Game/DungeonCrawlerContent/Blueprints/Inventory/InventoryItem.InventoryItem_C|GetItemName ItemToPickUp)) " has been picked up by " (Utilities|String|ToString(Name) (Variables|/Game/DungeonCrawlerContent/Blueprints/Characters/DCBaseCharacter.DCBaseCharacter_C|GetCharacterName (Variables|References|GetDCOwner)))) "NewEnumerator4")
          (Utilities|IsValid _gamegui
            (:Is%20Valid
              (Default|UpdateInventory _gamegui))))))))

(fn DropItem
  (params (ItemToDrop :type Inventory%20Item%20Object%20Reference))
  (bind _gamegui (Variables|References|GetGameGUI))
  (bind _statusfree (Default|CheckStatus (Variables|References|GetDCOwner) (Utilities|Struct|MakeStatus false false false false false false true)))
  (if _statusfree
    (Utilities|IsValid ItemToDrop
      (:Is%20Valid
        (switch Utilities|FlowControl|Switch|SwitchonItemStates (Variables|/Game/DungeonCrawlerContent/Blueprints/Inventory/InventoryItem.InventoryItem_C|GetItemState ItemToDrop)
          (:NewEnumerator1
            (Default|ChangeItemState ItemToDrop "NewEnumerator0")
            (Utilities|Array|RemoveItem (Variables|Default|GetInventory) ItemToDrop))
          (:NewEnumerator2
            (Default|ChangeItemState ItemToDrop "NewEnumerator0")
            (Utilities|Array|RemoveItem (Variables|Default|GetEquipment) ItemToDrop)
            (Default|Unequip ItemToDrop)))
        (Transformation|DetachFromActor ItemToDrop "KeepRelative" "KeepRelative" "KeepRelative")
        (Transformation|Teleport ItemToDrop (Math|Vector|MakeVector (.X (Math|Vector|BreakVector (.RandomLocation (Class|NavigationSystemV1|GetRandomPointinNavigableRadius (Transformation|GetActorLocation (Variables|References|GetDCOwner)) (Variables|Default|GetDropRadius) 0 0)))) (.Y (Math|Vector|BreakVector (.RandomLocation (Class|NavigationSystemV1|GetRandomPointinNavigableRadius (Transformation|GetActorLocation (Variables|References|GetDCOwner)) (Variables|Default|GetDropRadius) 0 0)))) (+ (.Z (Math|Vector|BreakVector (.RandomLocation (Class|NavigationSystemV1|GetRandomPointinNavigableRadius (Transformation|GetActorLocation (Variables|References|GetDCOwner)) (Variables|Default|GetDropRadius) 0 0)))) 1e+02)) (Math|Random|RandomRotator true))
        (Default|CallOnDropped ItemToDrop ItemToDrop)
        (Class|MessageInterface|SendMessage(Message) (Game|GetGameInstance) (Utilities|String|Append (Utilities|String|ToString(Name) (Variables|/Game/DungeonCrawlerContent/Blueprints/Inventory/InventoryItem.InventoryItem_C|GetItemName ItemToDrop)) " has been dropped by " (Utilities|String|ToString(Name) (Variables|/Game/DungeonCrawlerContent/Blueprints/Characters/DCBaseCharacter.DCBaseCharacter_C|GetCharacterName (Variables|References|GetDCOwner)))) "NewEnumerator4")
        (Variables|/Game/DungeonCrawlerContent/Blueprints/Inventory/InventoryItem.InventoryItem_C|SetDCOwner ItemToDrop 0)
        (Utilities|IsValid _gamegui
          (:Is%20Valid
            (Default|UpdateInventory _gamegui)))))))

(fn EquipItem
  (params (ItemToEquip :type Inventory%20Item%20Object%20Reference))
  (bind _dcowner (Variables|References|GetDCOwner))
  (bind _gamegui (Variables|References|GetGameGUI))
  (bind _itemtype (Variables|/Game/DungeonCrawlerContent/Blueprints/Inventory/InventoryItem.InventoryItem_C|GetItemType ItemToEquip))
  (bind _equipmentsockets (Variables|/Game/DungeonCrawlerContent/Blueprints/Characters/DCBaseCharacter.DCBaseCharacter_C|GetEquipmentSockets _dcowner))
  (bind (_weaponsocket _armoursocket _trinketsocket) (Utilities|Struct|BreakEquipmentSockets _equipmentsockets))
  (bind _statusfree (Default|CheckStatus (Variables|References|GetDCOwner) (Utilities|Struct|MakeStatus false false false false false false true)))
  (if _statusfree
    (Utilities|IsValid ItemToEquip
      (:Is%20Valid
        (switch Utilities|FlowControl|Switch|SwitchonItemStates (Variables|/Game/DungeonCrawlerContent/Blueprints/Inventory/InventoryItem.InventoryItem_C|GetItemState ItemToEquip)
          (:NewEnumerator0
            _)
          (:NewEnumerator1
            _))
        (bind _item (CallFunction|GetEquipment (Variables|/Game/DungeonCrawlerContent/Blueprints/Inventory/InventoryItem.InventoryItem_C|GetItemType ItemToEquip)))
        (Utilities|IsValid _item
          (:Is%20Valid
            (CallFunction|UnequipItem _item))
          (:Is%20Not%20Valid
            _))
        (Default|ChangeItemState ItemToEquip "NewEnumerator2")
        (Utilities|Array|RemoveItem (Variables|Default|GetInventory) ItemToEquip)
        (Utilities|Array|Insert (Variables|Default|GetEquipment) ItemToEquip (Math|Conversions|ToInteger(Byte) _itemtype))
        (switch Utilities|FlowControl|Switch|SwitchonItemType _itemtype
          (:NewEnumerator0
            (LocalVariables|SettempSocket _weaponsocket))
          (:NewEnumerator1
            (LocalVariables|SettempSocket _armoursocket))
          (:NewEnumerator2
            (LocalVariables|SettempSocket _trinketsocket)))
        (Transformation|AttachComponentToComponent ItemToEquip (Variables|/Script/Engine.Character|GetMesh (Variables|References|GetDCOwner)) (LocalVariables|GettempSocket) "SnapToTarget" "SnapToTarget" "SnapToTarget" true)
        (Default|Equip ItemToEquip)
        (Utilities|IsValid _gamegui
          (:Is%20Valid
            (Default|UpdateInventory _gamegui)))))))

(fn UnequipItem
  (params (ItemToUnEquip :type Inventory%20Item%20Object%20Reference))
  (bind _gamegui (Variables|References|GetGameGUI))
  (bind _statusfree (Default|CheckStatus (Variables|References|GetDCOwner) (Utilities|Struct|MakeStatus false false false false false false true)))
  (if _statusfree
    (Utilities|IsValid ItemToUnEquip
      (:Is%20Valid
        (switch Utilities|FlowControl|Switch|SwitchonItemStates (Variables|/Game/DungeonCrawlerContent/Blueprints/Inventory/InventoryItem.InventoryItem_C|GetItemState ItemToUnEquip)
          (:NewEnumerator2
            (Utilities|Array|RemoveItem (Variables|Default|GetEquipment) ItemToUnEquip)
            (Default|Unequip ItemToUnEquip)
            (Transformation|DetachFromActor ItemToUnEquip "KeepRelative" "KeepRelative" "KeepRelative")
            (if (< (Utilities|Array|Length (Variables|Default|GetInventory)) (Variables|Default|GetInventorySize))
              (CallFunction|PickUpItem ItemToUnEquip)
              (else
                (CallFunction|DropItem ItemToUnEquip)))
            (Utilities|IsValid _gamegui
              (:Is%20Valid
                (Default|UpdateInventory _gamegui)))))))))

(fn Init
  (Utilities|Array|Resize (Variables|Default|GetEquipment) 3)
  (CallFunction|SpawnStartingInventory))

(fn GetEquipment
  (params (ItemType :type ItemType%20Enum :default "NewEnumerator0"))
  (bind _returnvalue (Math|Conversions|ToInteger(Byte) ItemType))
  (bind _equipment (Variables|Default|GetEquipment))
  (bind _output (Utilities|Array|Get(acopy) _equipment _returnvalue))
  (Utilities|IsValid _output
    (:Is%20Valid
      (LocalVariables|SettempEquipment _output))
    (:Is%20Not%20Valid
      _))
  (return (LocalVariables|GettempEquipment)))

(fn SpawnStartingInventory
  (for _array_element (Variables|/Game/DungeonCrawlerContent/Blueprints/Characters/DCBaseCharacter.DCBaseCharacter_C|GetStartingEquipment (Variables|References|GetDCOwner))
    (bind _returnvalue (Game|SpawnActorfromClass _array_element (Math|Transform|MakeTransform "0, 0, 0" "0, 0, 0" "1.000000,1,1") "Undefined" 0 (Variables|References|GetDCOwner) 0))
    (Utilities|IsValid _returnvalue
      (:Is%20Valid
        (CallFunction|PickUpItem _returnvalue)
        (CallFunction|EquipItem _returnvalue))))
  (for _array_element_2 (Variables|/Game/DungeonCrawlerContent/Blueprints/Characters/DCBaseCharacter.DCBaseCharacter_C|GetStartingInventory (Variables|References|GetDCOwner))
    (bind _returnvalue_2 (Game|SpawnActorfromClass _array_element_2 (Math|Transform|MakeTransform "0, 0, 0" "0, 0, 0" "1.000000,1,1") "Undefined" 0 0 0))
    (Utilities|IsValid _returnvalue_2
      (:Is%20Valid
        (CallFunction|PickUpItem _returnvalue_2)))))

(fn ToggleEquipment
  (params (On :type Boolean))
  (bind _equipment (Variables|Default|GetEquipment))
  (if On
    (for _array_element _equipment
      (Utilities|IsValid _array_element
        (:Is%20Valid
          (Default|ChangeItemState _array_element "NewEnumerator2")
          (Default|HandleAttributeChanges _array_element true))))
    (else
      (for _array_element_2 _equipment
        (Utilities|IsValid _array_element_2
          (:Is%20Valid
            (Default|ChangeItemState _array_element_2 "NewEnumerator3")
            (Default|HandleAttributeChanges _array_element_2 false)))))))

(fn DropAllEquipment&Inventory
  (LocalVariables|SettempEquipment (Variables|Default|GetEquipment))
  (LocalVariables|SettempInventory (Variables|Default|GetInventory))
  (for _array_element (LocalVariables|GettempEquipment)
    (CallFunction|DropItem _array_element))
  (for _array_element_2 (LocalVariables|GettempInventory)
    (CallFunction|DropItem _array_element_2)))