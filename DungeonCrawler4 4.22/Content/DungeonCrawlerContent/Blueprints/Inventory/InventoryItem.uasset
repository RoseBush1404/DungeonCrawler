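; Inventory item actor for a dungeon crawler that can be dropped, picked up, equipped, used or switched off.
; ChangeItemState, also run at construction, sets mesh visibility, physics and collision per state, with only dropped items counting down a lifespan-based despawn.
; Equip and Unequip apply or reverse bonus and negative attributes on the owning character.
; Equip and use functions also fire event dispatchers and send messages through the game instance.
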(fn ConstructionScript
  (CallFunction|ChangeItemState (Variables|Default|GetItemState)))

(fn ChangeItemState
  (params (Equipped :type ItemStates%20Enum :default "NewEnumerator0"))
  (bind _mesh (Variables|Default|GetMesh))
  (bind _output_get (Variables|Default|SetItemState Equipped))
  (switch Utilities|FlowControl|Switch|SwitchonItemStates _output_get
    (:NewEnumerator0
      (Rendering|SetVisibility _mesh true true)
      (Physics|SetSimulatePhysics _mesh true)
      (Collision|SetCollisionEnabled (Variables|Default|GetEquippedCollision) "NoCollision")
      (Collision|SetCollisionEnabled _mesh "QueryAndPhysics")
      (Collision|SetCollisionResponsetoChannel _mesh "ECC_GameTraceChannel5" "ECR_Block")
      (CallFunction|HandleDespawntimer true))
    (:NewEnumerator1
      (Rendering|SetVisibility _mesh false true)
      (Physics|SetSimulatePhysics _mesh false)
      (Collision|SetCollisionEnabled (Variables|Default|GetEquippedCollision) "NoCollision")
      (Collision|SetCollisionEnabled _mesh "NoCollision")
      (Collision|SetCollisionResponsetoChannel _mesh "ECC_GameTraceChannel5" "ECR_Ignore")
      (CallFunction|HandleDespawntimer false))
    (:NewEnumerator2
      (Rendering|SetVisibility _mesh true true)
      (Physics|SetSimulatePhysics _mesh false)
      (Collision|SetCollisionEnabled _mesh "NoCollision")
      (Collision|SetCollisionEnabled _mesh "NoCollision")
      (Collision|SetCollisionResponsetoChannel _mesh "ECC_GameTraceChannel5" "ECR_Ignore")
      (CallFunction|HandleDespawntimer false))
    (:NewEnumerator3
      (Rendering|SetVisibility _mesh false true)
      (Physics|SetSimulatePhysics _mesh false)
      (Collision|SetCollisionEnabled (Variables|Default|GetEquippedCollision) "NoCollision")
      (Collision|SetCollisionEnabled _mesh "NoCollision")
      (Collision|SetCollisionResponsetoChannel _mesh "ECC_GameTraceChannel5" "ECR_Ignore")
      (CallFunction|HandleDespawntimer false)))
  (return true))

(fn StartUseItem
  (Default|CallOnUse self)
  (Class|MessageInterface|SendMessage(Message) (Game|GetGameInstance) (Utilities|String|Append (Utilities|String|ToString(Name) (Variables|Default|GetItemName)) " has been used by " (Utilities|String|ToString(Name) (Variables|/Game/DungeonCrawlerContent/Blueprints/Characters/DCBaseCharacter.DCBaseCharacter_C|GetCharacterName (Variables|Default|GetDCOwner)))) "NewEnumerator4")
  (return false))

(fn EndUseItem
  (Default|CallOnEndUse self)
  (Class|MessageInterface|SendMessage(Message) (Game|GetGameInstance) (Utilities|String|Append (Utilities|String|ToString(Name) (Variables|/Game/DungeonCrawlerContent/Blueprints/Characters/DCBaseCharacter.DCBaseCharacter_C|GetCharacterName (Variables|Default|GetDCOwner))) " ended using " (Utilities|String|ToString(Name) (Variables|Default|GetItemName))) "NewEnumerator4")
  (return false))

(fn Equip
  (CallFunction|HandleAttributeChanges true)
  (Default|CallOnEquip self)
  (Class|MessageInterface|SendMessage(Message) (Game|GetGameInstance) (Utilities|String|Append (Utilities|String|ToString(Name) (Variables|/Game/DungeonCrawlerContent/Blueprints/Characters/DCBaseCharacter.DCBaseCharacter_C|GetCharacterName (Variables|Default|GetDCOwner))) " started using " (Utilities|String|ToString(Name) (Variables|Default|GetItemName))) "NewEnumerator4")
  (return false))

(fn Unequip
  (CallFunction|HandleAttributeChanges false)
  (Default|CallOnUnequip self)
  (Class|MessageInterface|SendMessage(Message) (Game|GetGameInstance) (Utilities|String|Append (Utilities|String|ToString(Name) (Variables|Default|GetItemName)) " has been unequipped by " (Utilities|String|ToString(Name) (Variables|/Game/DungeonCrawlerContent/Blueprints/Characters/DCBaseCharacter.DCBaseCharacter_C|GetCharacterName (Variables|Default|GetDCOwner)))) "NewEnumerator4")
  (return false))

(fn HandleAttributeChanges
  (params (Equipping :type Boolean))
  (bind _dcowner (Variables|Default|GetDCOwner))
  (bind _dcowner_2 (Variables|Default|GetDCOwner))
  (if Equipping
    (Default|ModifyAttributes _dcowner (Variables|Default|GetBonusAttributes) true)
    (Default|ModifyAttributes _dcowner (Variables|Default|GetNegativeAttributes) false)
    (else
      (Default|ModifyAttributes _dcowner_2 (Variables|Default|GetBonusAttributes) false)
      (Default|ModifyAttributes _dcowner_2 (Variables|Default|GetNegativeAttributes) true))))

(fn HandleDespawntimer
  (params (Start :type Boolean))
  (if Start
    (Actor|SetLifeSpan (Variables|Default|GetDespawnTime))
    (else
      (Actor|SetLifeSpan 0.0))))

(fn GetName
  (return (Variables|Default|GetItemName)))