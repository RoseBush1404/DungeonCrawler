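; Effect manager actor that tracks the status effects on an owning actor (DCOwner), each a spawned actor, and destroys them and itself when the owner ends play.
; Adding an effect stacks an existing one of the same class or spawns a new one, up to a maximum count.
; Before adds and after removals, it ends and restarts every stack to refresh effects.
; Dispatchers announce changes, and bulk removal can spare persistent effects.
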(event Custom|DCOwnerEndPlay
  (params (Actor :type Actor%20Object%20Reference) (EndPlayReason :type EEndPlayReason%20Enum :default "Destroyed"))
  (for _array_element (Variables|Default|GetEffects)
    (Actor|DestroyActor _array_element))
  (Actor|DestroyActor))

(event EventBeginPlay
  (Game|AssignOnEndPlay (Variables|References|GetDCOwner) (delegate Custom|DCOwnerEndPlay)))

(fn ConstructionScript)

(fn AddEffect
  (params (EffectClass :type Effect%20Class%20Reference) (Inciter :type DC%20Base%20Character%20Object%20Reference))
  (if (< (Utilities|Array|Length (Variables|Default|GetEffects)) (Variables|Default|GetMaxEffects))
    (CallFunction|RefreshEffects)
    (bind _effectinstack (CallFunction|CheckifEffectExists EffectClass))
    (Utilities|IsValid _effectinstack
      (:Is%20Valid
        (Default|ModifyStacks _effectinstack 1 true Inciter)
        (LocalVariables|SettempEffect _effectinstack)
        (Default|CallOnModifyStacks))
      (:Is%20Not%20Valid
        (bind _returnvalue (Game|SpawnActorfromClass EffectClass (Math|Transform|MakeTransform "0, 0, 0") "Undefined" 0 (Variables|References|GetDCOwner) self 0))
        (Utilities|Array|Add (Variables|Default|GetEffects) _returnvalue)
        (LocalVariables|SettempEffect _returnvalue)
        (Default|InitEffect _returnvalue Inciter)
        (Default|CallOnAddEffect self _returnvalue)))
    (return (LocalVariables|GettempEffect))))

(fn RemoveEffect
  (params (Effect :type Effect%20Object%20Reference))
  (Utilities|IsValid Effect
    (:Is%20Valid
      (Default|TerminateEffect Effect)
      (Utilities|Array|RemoveItem (Variables|Default|GetEffects) Effect)
      (CallFunction|RefreshEffects)
      (Default|CallOnRemoveEffect self Effect)
      (Actor|DestroyActor Effect))))

(fn RemoveAllEffects
  (params (RemovePersistent :type Boolean))
  (bind _effects (Variables|Default|GetEffects))
  (if RemovePersistent
    (LocalVariables|SettempEffects _effects)
    (for _array_element (LocalVariables|GettempEffects) :!label _label
      (CallFunction|RemoveEffect _array_element))
    (else
      (for _array_element_2 _effects
        (bind _ispersistent (Default|CheckPersistent _array_element_2))
        (if (not _ispersistent)
          (Utilities|Array|Add (LocalVariables|GettempEffects) _array_element_2)
          (goto _label))))))

(fn CheckifEffectExists
  (params (EffectToCheck :type Effect%20Class%20Reference))
  (for _array_element (Variables|Default|GetEffects)
    (if (== (Utilities|GetClass _array_element) EffectToCheck)
      (return _array_element)))
  (return 0))

(fn RefreshEffects
  (bind _effects (Variables|Default|GetEffects))
  (bind _output_get (LocalVariables|SettempEffects _effects))
  (Utilities|Array|Clear _effects)
  (for _array_element _output_get
    (Utilities|Array|Add (LocalVariables|Getincitors) (Variables|/Game/DungeonCrawlerContent/Blueprints/Effects/Effect.Effect_C|GetIncitor _array_element))
    (for _index (range 1 (Variables|/Game/DungeonCrawlerContent/Blueprints/Effects/Effect.Effect_C|GetStacks _array_element))
      (Default|EndEffect _array_element)))
  (for (_array_element_2 _array_index) (LocalVariables|GettempEffects)
    (Utilities|Array|AddUnique (Variables|Default|GetEffects) _array_element_2)
    (for _index_2 (range 1 (Variables|/Game/DungeonCrawlerContent/Blueprints/Effects/Effect.Effect_C|GetStacks _array_element_2))
      (Default|StartEffect _array_element_2 (Utilities|Array|Get(acopy) (LocalVariables|Getincitors) _array_index)))))

(fn GetEffectOfClass
  (params (EffectClass :type Effect%20Class%20Reference))
  (if (Utilities|IsValidClass EffectClass)
    (for _array_element (Variables|Default|GetEffects)
      (if (== (Utilities|GetClass _array_element) EffectClass)
        (LocalVariables|SetTempEffect _array_element)))
    (Utilities|IsValid (LocalVariables|GetTempEffect)
      (:Is%20Valid
        (return true (LocalVariables|GetTempEffect)))
      (:Is%20Not%20Valid
        (return false 0)))
    (else
      (return false 0))))