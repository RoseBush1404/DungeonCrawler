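; Base status effect for a dungeon crawler: a stackable, optionally timed effect applied to a character by an inciter.
; Init and terminate run StartEffect and EndEffect per stack; starting attaches a particle emitter, and both broadcast events and game messages.
; A duration timer asks the owning manager to remove the effect, while zero or negative durations persist.
; Stack changes clamp the count and restart the timer, calling StartEffect even on decreases.
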(fn ConstructionScript)

(fn InitEffect
  (params (Inciter :type DC%20Base%20Character%20Object%20Reference))
  (for _index (range 1 (Variables|Attributes|GetStacks))
    (CallFunction|StartEffect Inciter))
  (CallFunction|InitEffectTimer)
  (return true))

(fn TerminateEffect
  (bind _spawnedemitter (Variables|FX|GetSpawnedEmitter))
  (for _index (range 1 (Variables|Attributes|GetStacks))
    (CallFunction|EndEffect))
  (Default|CallOnEndEffect self)
  (Variables|Default|SetIncitor 0)
  (Utilities|IsValid _spawnedemitter
    (:Is%20Valid
      (Components|DestroyComponent _spawnedemitter))
    (:Is%20Not%20Valid
      _))
  (Class|MessageInterface|SendMessage(Message) (Game|GetGameInstance) (Utilities|String|Append (Utilities|String|ToString(Name) (Variables|Attributes|GetEffectName)) " has ended on " (Utilities|String|ToString(Name) (Variables|/Game/DungeonCrawlerContent/Blueprints/Characters/DCBaseCharacter.DCBaseCharacter_C|GetCharacterName (Variables|References|GetDCOwner)))) "NewEnumerator2"))

(fn StartEffect
  (params (Incitor :type DC%20Base%20Character%20Object%20Reference))
  (bind _effectfx (Variables|FX|GetEffectFX))
  (bind _dcowner (Variables|References|GetDCOwner))
  (Utilities|IsValid (Variables|Default|GetIncitor)
    (:Is%20Valid
      (if (== (Variables|Default|GetIncitor) Incitor)
        (Variables|Default|SetIncitor Incitor :!label _label)
        (Default|CallOnStartEffect self)
        (Variables|Default|SetIncitorAttributes (Variables|/Game/DungeonCrawlerContent/Blueprints/Characters/DCBaseCharacter.DCBaseCharacter_C|GetAttributes Incitor))
        (Utilities|IsValid _effectfx
          (:Is%20Valid
            (Utilities|IsValid (Variables|FX|GetSpawnedEmitter)
              (:Is%20Valid
                (Components|DestroyComponent (Variables|FX|GetSpawnedEmitter)))
              (:Is%20Not%20Valid
                _))
            (bind _returnvalue (Effects|SpawnEmitterAttached _effectfx (Variables|/Script/Engine.Character|GetMesh _dcowner) "None" (Transformation|GetActorLocation _dcowner) "0, 0, 0" "1.000000,1.000000,1.000000" "KeepWorldPosition"))
            (Variables|FX|SetSpawnedEmitter _returnvalue))
          (:Is%20Not%20Valid
            _))
        (Class|MessageInterface|SendMessage(Message) (Game|GetGameInstance) (Utilities|String|Append (Utilities|String|ToString(Name) (Variables|Attributes|GetEffectName)) " has been started on " (Utilities|String|ToString(Name) (Variables|/Game/DungeonCrawlerContent/Blueprints/Characters/DCBaseCharacter.DCBaseCharacter_C|GetCharacterName (Variables|References|GetDCOwner)))) "NewEnumerator2")
        (return true)))
    (:Is%20Not%20Valid
      (goto _label))))

(fn EndEffect
  (return true))

(fn InitEffectTimer
  (bind _ispersistent (CallFunction|CheckPersistent))
  (if (not _ispersistent)
    (if (Utilities|Time|IsTimerActivebyHandle (Variables|Timers|GetDurationTimerHandle))
      (Utilities|Time|ClearandInvalidateTimerbyHandle (Variables|Timers|GetDurationTimerHandle)))
    (bind _returnvalue (Utilities|Time|SetTimerbyFunctionName 0 "EndEffectTimer" (Variables|Attributes|GetDuration)))
    (Variables|Timers|SetDurationTimerHandle _returnvalue)))

(fn CheckPersistent
  (return (<= (Variables|Attributes|GetDuration) 0.0)))

(fn ModifyStacks
  (params (Amount :type Integer) (Positive :type Boolean) (Incitor :type DC%20Base%20Character%20Object%20Reference))
  (bind _returnvalue (Math|Integer|Absolute(Integer) Amount))
  (if Positive
    (LocalVariables|SettempStacks (+ (Variables|Attributes|GetStacks) _returnvalue))
    (if (>= (Variables|Attributes|GetStacks) (Variables|Attributes|GetMaxStacks))
      _
      (else
        (Variables|Attributes|SetStacks (Math|Integer|Clamp(Integer) (LocalVariables|GettempStacks) 1 (Variables|Attributes|GetMaxStacks)) :!label _label)
        (CallFunction|StartEffect Incitor)))
    (else
      (LocalVariables|SettempStacks (- (Variables|Attributes|GetStacks) _returnvalue))
      (goto _label)))
  (CallFunction|InitEffectTimer)
  (Default|CallOnModifyStack self (Variables|Attributes|GetStacks)))

(fn EndEffectTimer
  (Default|RemoveEffect (Variables|References|GetOwningManager) self))

(fn GetName
  (return (Variables|Attributes|GetEffectName)))