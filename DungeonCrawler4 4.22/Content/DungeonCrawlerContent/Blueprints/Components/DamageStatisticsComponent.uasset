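; Component that records damage statistics per named damage source for its owning character, like a damage meter.
; Damage and critical events add damage, hits and crits to running totals, firing events when new sources appear.
; Combat start clears per-combat maps and starts a looping timer that recomputes each source's DPS from combat damage over elapsed time and broadcasts a tick.
; Combat end stops the timer.
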(event Custom|Init
  (bind _owningcharacter (Variables|Default|GetOwningCharacter))
  (EventDispatchers|AssignOnCauseDamage _owningcharacter (EventDispatchers|CreateEvent :!event Custom|OnDamage))
  (EventDispatchers|AssignOnCritical _owningcharacter (EventDispatchers|CreateEvent :!event Custom|OnCrit))
  (EventDispatchers|AssignOnStartCombat _owningcharacter (EventDispatchers|CreateEvent :!event Custom|StartCombat))
  (EventDispatchers|AssignOnEndCombat _owningcharacter (EventDispatchers|CreateEvent :!event Custom|EndCombat)))

(event Custom|StartCombat
  (params (ID :type DC%20Base%20Character%20Object%20Reference))
  (Utilities|Map|Clear (Variables|Default|GetDamageThisCombat))
  (Utilities|Map|Clear (Variables|Default|GetDPSThisCombat))
  (Variables|Default|SetInCombat true)
  (bind _returnvalue (Utilities|Time|SetTimerbyFunctionName 0 "CombatTime" (Variables|Default|GetCombatTimeTick) true))
  (Variables|Default|SetCombatTimer _returnvalue))

(event Custom|EndCombat
  (params (ID :type DC%20Base%20Character%20Object%20Reference))
  (Variables|Default|SetInCombat false)
  (Utilities|Time|ClearandInvalidateTimerbyHandle (Variables|Default|GetCombatTimer))
  (Variables|Default|SetTimeInCombat 0.0))

(event Custom|CombatTime
  (Variables|Default|SetTimeInCombat (+ (Variables|Default|GetTimeInCombat) (Variables|Default|GetCombatTimeTick)))
  (Default|CallOnCombatTick self)
  (bind _keys (Utilities|Map|Keys (Variables|Default|GetDamageThisCombat)))
  (for _array_element _keys
    (Utilities|Map|Add (Variables|Default|GetDPSThisCombat) _array_element (/ (Math|Conversions|ToFloat(Integer) (.Value (Utilities|Map|Find (Variables|Default|GetDamageThisCombat) _array_element))) (Variables|Default|GetTimeInCombat)))
    (Utilities|Map|Add (Variables|Default|GetDamageSourceStats) _array_element (Utilities|Struct|MakeDamageStatistics (.Damage (Utilities|Struct|BreakDamageStatistics (.Value (Utilities|Map|Find (Variables|Default|GetDamageSourceStats) _array_element)))) (/ (Math|Conversions|ToFloat(Integer) (.Value (Utilities|Map|Find (Variables|Default|GetDamageThisCombat) _array_element))) (Variables|Default|GetTimeInCombat)) (.Hits (Utilities|Struct|BreakDamageStatistics (.Value (Utilities|Map|Find (Variables|Default|GetDamageSourceStats) _array_element)))) (.AverageHit (Utilities|Struct|BreakDamageStatistics (.Value (Utilities|Map|Find (Variables|Default|GetDamageSourceStats) _array_element)))) (.Crits (Utilities|Struct|BreakDamageStatistics (.Value (Utilities|Map|Find (Variables|Default|GetDamageSourceStats) _array_element)))) (.AverageCrits (Utilities|Struct|BreakDamageStatistics (.Value (Utilities|Map|Find (Variables|Default|GetDamageSourceStats) _array_element))))))))

(event Custom|OnDamage
  (params (ID :type DC%20Base%20Character%20Object%20Reference) (Damage :type Integer) (Target :type DC%20Base%20Character%20Object%20Reference) (DamageSource :type Actor%20Object%20Reference) (DamageType :type Damage%20Type%20Class%20Reference))
  (Utilities|IsValid DamageSource
    (:Is%20Valid
      (bind _name (Class|NameInterface|GetName(Message) DamageSource))
      (CallFunction|UpdateDamageSource (Utilities|String|ToString(Name) _name) (Utilities|Struct|MakeDamageStatistics Damage 0.0 1 0.0 0 0.0))
      (if (Variables|Default|GetInCombat)
        (if (.ReturnValue (Utilities|Map|Find (Variables|Default|GetDamageThisCombat) (Utilities|String|ToString(Name) _name)))
          _
          (else
            (Default|CallOnNewDamageSourceThisCombat self (Utilities|String|ToString(Name) _name))))
        (Utilities|Map|Add (Variables|Default|GetDamageThisCombat) (Utilities|String|ToString(Name) _name) (+ (.Value (Utilities|Map|Find (Variables|Default|GetDamageThisCombat) (Utilities|String|ToString(Name) _name))) Damage))))))

(event Custom|OnCrit
  (params (ID :type DC%20Base%20Character%20Object%20Reference) (Source :type Actor%20Object%20Reference))
  (bind _name (Class|NameInterface|GetName(Message) Source))
  (CallFunction|UpdateDamageSource (Utilities|String|ToString(Name) _name) (Utilities|Struct|MakeDamageStatistics 0 0.0 0 0.0 1 0.0)))

(fn UpdateDamageSource
  (params (Source :type String) (DamageStats :type Damage%20Statistics%20Structure))
  (bind (_damage _dps _hits _averagehit _crits _averagecrits) (Utilities|Struct|BreakDamageStatistics DamageStats))
  (bind _damagesourcestats (Variables|Default|GetDamageSourceStats))
  (bind (_value _returnvalue) (Utilities|Map|Find _damagesourcestats Source))
  (bind (_damage_2 _dps_2 _hits_2 _averagehit_2 _crits_2 _averagecrits_2) (Utilities|Struct|BreakDamageStatistics _value))
  (if _returnvalue
    _
    (else
      (Default|CallOnNewDamageSource self Source)))
  (Utilities|Map|Add (Variables|Default|GetDamageSourceStats) Source (Utilities|Struct|MakeDamageStatistics (+ _damage_2 _damage) (+ _dps_2 _dps) (+ _hits_2 _hits) (+ _averagehit_2 _averagehit) (+ _crits_2 _crits) (+ _averagecrits_2 _averagecrits))))