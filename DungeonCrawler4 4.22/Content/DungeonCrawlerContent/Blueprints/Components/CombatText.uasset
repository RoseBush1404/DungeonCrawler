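; Component that shows floating combat text for its owning character when combat events occur.
; Init binds handlers to the character's take damage, critical, disable, immobilise, invulnerable, silence and level-up dispatchers.
; Each handler creates a new CombatTextWidget for the affected character with its own text, colour and offset, then adds it to the viewport.
; Damage displays the numeric amount, while the other events display fixed labels.
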(event Custom|OnTakeDamageEvent
  (params (ID :type DC%20Base%20Character%20Object%20Reference) (Damage :type Integer) (DamagingCharacter :type DC%20Base%20Character%20Object%20Reference) (DamageSource :type Actor%20Object%20Reference))
  (bind _returnvalue (UserInterface|CreateWidget "/Game/DungeonCrawlerContent/Blueprints/UI/Widgets/CombatTextWidget.CombatTextWidget_C" 0 ID (Utilities|Text|ToText(Integer) Damage) (Utilities|Struct|MakeSlateColor "(R=1.000000,G=0.987742,B=0.000000,A=1.000000)") "0.000000,-20.000000,100.000000" "Forward"))
  (UserInterface|Viewport|AddtoViewport _returnvalue 0))

(event Custom|OnDisableEvent
  (params (ID :type DC%20Base%20Character%20Object%20Reference) (Duration :type Float%20%28single-precision%29) (Source :type Actor%20Object%20Reference))
  (bind _returnvalue (UserInterface|CreateWidget "/Game/DungeonCrawlerContent/Blueprints/UI/Widgets/CombatTextWidget.CombatTextWidget_C" 0 ID "Disabled" (Utilities|Struct|MakeSlateColor "(R=1.000000,G=0.068713,B=0.633029,A=1.000000)") "0.000000,-50.000000,100.000000" "Forward"))
  (UserInterface|Viewport|AddtoViewport _returnvalue 0))

(event Custom|OnImmobaliseEvent
  (params (ID :type DC%20Base%20Character%20Object%20Reference) (Duration :type Float%20%28single-precision%29) (Source :type Actor%20Object%20Reference))
  (bind _returnvalue (UserInterface|CreateWidget "/Game/DungeonCrawlerContent/Blueprints/UI/Widgets/CombatTextWidget.CombatTextWidget_C" 0 ID "Immobalised" (Utilities|Struct|MakeSlateColor "(R=0.000000,G=1.000000,B=0.290900,A=1.000000)") "0.000000,-65.000000,100.000000" "Forward"))
  (UserInterface|Viewport|AddtoViewport _returnvalue 0))

(event Custom|OnInvulnerableEvent
  (params (ID :type DC%20Base%20Character%20Object%20Reference) (Duration :type Float%20%28single-precision%29) (Source :type Actor%20Object%20Reference))
  (bind _returnvalue (UserInterface|CreateWidget "/Game/DungeonCrawlerContent/Blueprints/UI/Widgets/CombatTextWidget.CombatTextWidget_C" 0 ID "Invulnerable" (Utilities|Struct|MakeSlateColor "(R=0.000000,G=0.076538,B=1.000000,A=1.000000)") "0.000000,-65.000000,100.000000" "Forward"))
  (UserInterface|Viewport|AddtoViewport _returnvalue 0))

(event Custom|Init
  (EventDispatchers|AssignOnTakeDamage (Variables|Default|GetOwningCharacter) (delegate Custom|OnTakeDamageEvent))
  (EventDispatchers|AssignOnCritical (Variables|Default|GetOwningCharacter) (delegate Custom|OnCriticalEvent))
  (EventDispatchers|AssignOnDisable (Variables|Default|GetOwningCharacter) (delegate Custom|OnDisableEvent))
  (EventDispatchers|AssignOnImmobalise (Variables|Default|GetOwningCharacter) (delegate Custom|OnImmobaliseEvent))
  (EventDispatchers|AssignOnInvulnerable (Variables|Default|GetOwningCharacter) (delegate Custom|OnInvulnerableEvent))
  (EventDispatchers|AssignOnSilence (Variables|Default|GetOwningCharacter) (delegate Custom|OnSilenceEvent))
  (EventDispatchers|AssignOnLevelUp (Variables|Default|GetOwningCharacter) (delegate Custom|OnLevelUpEvent)))

(event Custom|OnSilenceEvent
  (params (ID :type DC%20Base%20Character%20Object%20Reference) (Duration :type Float%20%28single-precision%29) (Source :type Actor%20Object%20Reference))
  (bind _returnvalue (UserInterface|CreateWidget "/Game/DungeonCrawlerContent/Blueprints/UI/Widgets/CombatTextWidget.CombatTextWidget_C" 0 ID "Silenced" (Utilities|Struct|MakeSlateColor "(R=0.395369,G=0.090642,B=1.000000,A=1.000000)") "0.000000,-50.000000,100.000000" "Forward"))
  (UserInterface|Viewport|AddtoViewport _returnvalue 0))

(event Custom|OnLevelUpEvent
  (params (ID :type DC%20Base%20Character%20Object%20Reference))
  (bind _returnvalue (UserInterface|CreateWidget "/Game/DungeonCrawlerContent/Blueprints/UI/Widgets/CombatTextWidget.CombatTextWidget_C" 0 ID "Level Up" (Utilities|Struct|MakeSlateColor "(R=0.386756,G=1.000000,B=0.012887,A=1.000000)") "0.000000,-50.000000,100.000000" "Forward"))
  (UserInterface|Viewport|AddtoViewport _returnvalue 0))

(event Custom|OnCriticalEvent
  (params (ID :type DC%20Base%20Character%20Object%20Reference) (Source :type Actor%20Object%20Reference))
  (bind _returnvalue (UserInterface|CreateWidget "/Game/DungeonCrawlerContent/Blueprints/UI/Widgets/CombatTextWidget.CombatTextWidget_C" 0 ID "Critical" (Utilities|Struct|MakeSlateColor "(R=1.000000,G=0.118750,B=0.000000,A=1.000000)") "0.000000,-50.000000,100.000000" "Forward"))
  (UserInterface|Viewport|AddtoViewport _returnvalue 0))