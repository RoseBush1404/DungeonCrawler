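; Dungeon crawler projectile actor that destroys itself on a collision hit and reports valid overlaps.
; Overlaps require a valid owner and ignore it; without the game mode's friendly fire, only characters on another TeamID count.
; Accepted overlaps go to Overlaped, which fires the OnOverlapped dispatcher and sends a message naming both parties to the game instance.
; It applies no damage itself, and Init is empty.
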(event OnComponentBeginOverlap(Collision)
  (params (OverlappedComponent :type Primitive%20Component%20Object%20Reference) (OtherActor :type Actor%20Object%20Reference) (OtherComp :type Primitive%20Component%20Object%20Reference) (OtherBodyIndex :type Integer) (bFromSweep :type Boolean) (SweepResult :type Hit%20Result%20Structure%20%28by%20ref%29))
  (bind _dcowner (Variables|Default|GetDCOwner))
  (Utilities|IsValid _dcowner
    (:Is%20Valid
      (if (!= OtherActor _dcowner)
        (bind _gamemodedata (Class|GameModeInterface|GetGameModeData(Message) (Game|GetGameMode)))
        (if (Utilities|Struct|BreakGameModeData _gamemodedata)
          (CallFunction|Overlaped OtherActor :!label _label)
          (else
            (bind _asdcbase_character (Utilities|Casting|CastToDCBaseCharacter OtherActor))
            (if (!= (Variables|/Game/DungeonCrawlerContent/Blueprints/Characters/DCBaseCharacter.DCBaseCharacter_C|GetTeamID _asdcbase_character) (Variables|/Game/DungeonCrawlerContent/Blueprints/Characters/DCBaseCharacter.DCBaseCharacter_C|GetTeamID (Variables|Default|GetDCOwner)))
              (goto _label))))))))

(event OnComponentHit(Collision)
  (params (HitComponent :type Primitive%20Component%20Object%20Reference) (OtherActor :type Actor%20Object%20Reference) (OtherComp :type Primitive%20Component%20Object%20Reference) (NormalImpulse :type Vector :default "0, 0, 0") (Hit :type Hit%20Result%20Structure%20%28by%20ref%29))
  (Actor|DestroyActor))

(fn ConstructionScript)

(fn Init)

(fn Overlaped
  (params (Actor :type Actor%20Object%20Reference))
  (Default|CallOnOverlapped self Actor)
  (Class|MessageInterface|SendMessage(Message) (Game|GetGameInstance) (Utilities|String|Append (Utilities|String|ToString(Name) (Variables|Default|GetProjectileName)) " has overlapped with " (Utilities|GetDisplayName Actor)) "NewEnumerator8")
  (return true))

(fn GetName
  (return (Variables|Default|GetProjectileName)))