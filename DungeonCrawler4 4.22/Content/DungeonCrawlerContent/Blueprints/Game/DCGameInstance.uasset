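; Game instance for the dungeon crawler that serves as a central debug message channel and exposes GameData through a getter.
; SendMessage routes text to PrintMessage, which prints it on screen in a colour chosen by message type, only if that type's filter flag is on.
; FilterMessageChannel flips a type's flag in the MessageFilters array, indexed by the enum value, and prints the channel's new state.
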(event EventFilterMessageChannel
  (params (Type :type MessageType%20Enum :default "NewEnumerator6"))
  ;[1 1 1] Messages
  (CallFunction|FilterMessageType Type))

(event EventSendMessage
  (params (Message :type String) (Type :type MessageType%20Enum :default "NewEnumerator6"))
  ;[1 1 1] Messages
  (CallFunction|PrintMessage Message Type))

(fn FilterMessageType
  (params (Type :type MessageType%20Enum :default "NewEnumerator6"))
  (bind _returnvalue (Math|Conversions|ToInteger(Byte) Type))
  (bind _messagefilters (Variables|Default|GetMessageFilters))
  (bind _output (Utilities|Array|Get(acopy) _messagefilters _returnvalue))
  (Utilities|Array|SetArrayElem _messagefilters _returnvalue (not _output))
  (if _output
    (LocalVariables|SettempToggleString "on.")
    (else
      (LocalVariables|SettempToggleString "off.")))
  (Development|PrintString (Utilities|String|Append (Utilities|String|EnumtoString Type) " chanel has been toggled " (LocalVariables|GettempToggleString)) true true "(R=0.000000,G=0.660000,B=1.000000,A=1.000000)" 5.0))

(fn PrintMessage
  (params (Message :type String) (Type :type MessageType%20Enum :default "NewEnumerator6"))
  (bind _returnvalue (Math|Conversions|ToInteger(Byte) Type))
  (bind _messagefilters (Variables|Default|GetMessageFilters))
  (bind _output (Utilities|Array|Get(acopy) _messagefilters _returnvalue))
  (switch Utilities|FlowControl|Switch|SwitchonMessageType Type
    (:NewEnumerator6
      (if _output
        (LocalVariables|SettempColour "(R=0.277217,G=0.000000,B=1.000000,A=1.000000)")
        (LocalVariables|SettempDuration 2.0)
        (Development|PrintString Message true true (LocalVariables|GettempColour) (LocalVariables|GettempDuration) :!label _label)))
    (:NewEnumerator7
      (if _output
        (LocalVariables|SettempColour "(R=1.000000,G=0.000000,B=0.017050,A=1.000000)")
        (LocalVariables|SettempDuration 2.0)
        (goto _label)))
    (:NewEnumerator4
      (if _output
        (LocalVariables|SettempColour "(R=0.000000,G=0.851736,B=1.000000,A=1.000000)")
        (LocalVariables|SettempDuration 2.0)
        (goto _label)))
    (:NewEnumerator1
      (if _output
        (LocalVariables|SettempColour "(R=0.000000,G=1.000000,B=0.068148,A=1.000000)")
        (LocalVariables|SettempDuration 2.0)
        (goto _label)))
    (:NewEnumerator2
      (if _output
        (LocalVariables|SettempColour "(R=1.000000,G=0.913040,B=0.000000,A=1.000000)")
        (LocalVariables|SettempDuration 2.0)
        (goto _label)))
    (:NewEnumerator3
      (if _output
        (LocalVariables|SettempColour "(R=1.000000,G=0.157706,B=0.000000,A=1.000000)")
        (LocalVariables|SettempDuration 2.0)
        (goto _label)))
    (:NewEnumerator8
      (if _output
        (LocalVariables|SettempColour "(R=0.000000,G=0.022420,B=1.000000,A=1.000000)")
        (LocalVariables|SettempDuration 2.0)
        (goto _label)))
    (:NewEnumerator5
      (if _output
        (LocalVariables|SettempColour "(R=0.995000,G=0.000000,B=0.726662,A=1.000000)")
        (LocalVariables|SettempDuration 2.0)
        (goto _label)))))

(fn GetGameData
  (return (Variables|Default|GetGameData)))