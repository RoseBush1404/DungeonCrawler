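; Base ability for a dungeon crawler character (DCOwner), handling use checks, resource cost, cooldown and skill level.
; UseAbility validates owner status, resource and cooldown, plus target range for targeted types, and only reports success.
; ExecuteAbility separately ends casting, spends resource, fires a dispatcher and sends a game-instance message, leaving a placeholder for ability effects.
; StartCooldown runs a reset timer using a clamped cooldown derived from the owner's cooldown reduction.
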(event EventBeginPlay
  (Variables|Attributes|SetCooldown (Variables|Attributes|GetBaseCooldown)))

(fn ConstructionScript)

(fn UseAbility
  (params (Target :type DC%20Base%20Character%20Object%20Reference))
  (bind _dcowner (Variables|References|GetDCOwner))
  (bind _returnvalue (Transformation|GetDistanceTo Target _dcowner))
  (bind _useable (CallFunction|CheckUseable))
  (if _useable
    (if (Variables|Handelers|GetOnCooldown)
      _
      (else
        (switch Utilities|FlowControl|Switch|SwitchonAbilityType (Variables|Default|GetType)
          (:NewEnumerator1
            (LocalVariables|SetSuccess true :!label _label))
          (:NewEnumerator0
            (Utilities|IsValid Target
              (:Is%20Valid
                (if (and (>= _returnvalue (Variables|Default|GetMinRange)) (<= _returnvalue (Variables|Default|GetMaxRange)))
                  (Variables|Default|SetTarget Target)
                  (goto _label)
                  (else
                    _)))))))))
  (return (LocalVariables|GetSuccess)))

(fn ResetCooldown
  (Variables|Handelers|SetOnCooldown false)
  (Utilities|Time|ClearandInvalidateTimerbyHandle (Variables|Timers|GetCooldownTimerHandle)))

(fn ExecuteAbility
  (bind _dcowner (Variables|References|GetDCOwner))
  ;[1 1 1] Ability Functionality
  (Default|EndCasting _dcowner)
  (Default|ModifyResource _dcowner (Variables|Attributes|GetResourceCost) false)
  (Default|CallOnExecuteAbility self)
  (Class|MessageInterface|SendMessage(Message) (Game|GetGameInstance) (Utilities|String|Append (Utilities|String|ToString(Name) (Variables|/Game/DungeonCrawlerContent/Blueprints/Characters/DCBaseCharacter.DCBaseCharacter_C|GetCharacterName (Variables|References|GetDCOwner))) " has used " (Utilities|String|ToString(Name) (Variables|Attributes|GetAbilityName))) "NewEnumerator1")
  (return true))

(fn ModifyBaseCooldown
  (params (Amount :type Float%20%28single-precision%29) (Positive :type Boolean))
  (bind _returnvalue (Math|Float|Absolute(Float) Amount))
  (if Positive
    (LocalVariables|SettempCooldown (+ _returnvalue (Variables|Attributes|GetBaseCooldown)))
    (else
      (LocalVariables|SettempCooldown (- (Variables|Attributes|GetBaseCooldown) _returnvalue))))
  (Variables|Attributes|SetBaseCooldown (Math|Float|Clamp(Float) (LocalVariables|GettempCooldown) 0.1 1e+03))
  (CallFunction|SetCooldownfromPercentage (.CooldownReduction (Utilities|Struct|BreakCharacterAttributes (Variables|/Game/DungeonCrawlerContent/Blueprints/Characters/DCBaseCharacter.DCBaseCharacter_C|GetAttributes (Variables|References|GetDCOwner))))))

(fn SetCooldownfromPercentage
  (params (CooldownReduction :type Float%20%28single-precision%29))
  (Variables|Attributes|SetCooldown (Math|Float|Clamp(Float) (Utilities|CalculateCooldownReduction (Variables|Attributes|GetBaseCooldown) CooldownReduction) 0.1 1e+03)))

(fn ModifyCooldown
  (params (Amount :type Float%20%28single-precision%29) (Positive :type Boolean))
  (bind _returnvalue (Math|Float|Absolute(Float) Amount))
  (if Positive
    (LocalVariables|SettempCooldown (+ _returnvalue (Variables|Attributes|GetCooldown)))
    (else
      (LocalVariables|SettempCooldown (- (Variables|Attributes|GetCooldown) _returnvalue))))
  (Variables|Attributes|SetCooldown (Math|Float|Clamp(Float) (LocalVariables|GettempCooldown) 0.1 (Variables|Attributes|GetBaseCooldown))))

(fn StartCooldown
  (bind _returnvalue (Utilities|Time|SetTimerbyFunctionName 0 "ResetCooldown" (Variables|Attributes|GetCooldown)))
  (Variables|Timers|SetCooldownTimerHandle _returnvalue)
  (Variables|Handelers|SetOnCooldown true)
  (Variables|Default|SetTarget 0))

(fn Init
  (CallFunction|SetCooldownfromPercentage (Utilities|Struct|BreakCharacterAttributes (Variables|/Game/DungeonCrawlerContent/Blueprints/Characters/DCBaseCharacter.DCBaseCharacter_C|GetAttributes (Variables|References|GetDCOwner))))
  (CallFunction|ResetCooldown)
  (return false))

(fn CheckUseable
  (bind _dcowner (Variables|References|GetDCOwner))
  (bind _statusfree (Default|CheckStatus _dcowner (Utilities|Struct|MakeStatus true true false true false true true)))
  (return (and _statusfree (> (- (Utilities|Struct|BreakCharacterAttributes (Variables|/Game/DungeonCrawlerContent/Blueprints/Characters/DCBaseCharacter.DCBaseCharacter_C|GetAttributes _dcowner)) (Variables|Attributes|GetResourceCost)) 0))))

(fn Reset
  (CallFunction|ResetCooldown)
  (Variables|Default|SetTarget 0)
  (return true))

(fn SkillUp
  (Default|CallOnSkillUp self)
  (Math|Integer|IncrementInt (Variables|Default|GetSkillLevel)
    (:%20%20
      (Class|MessageInterface|SendMessage(Message) (Game|GetGameInstance) (Utilities|String|Append (Utilities|String|ToString(Name) (Variables|/Game/DungeonCrawlerContent/Blueprints/Characters/DCBaseCharacter.DCBaseCharacter_C|GetCharacterName (Variables|References|GetDCOwner))) "'s " (Utilities|String|ToString(Name) (Variables|Attributes|GetAbilityName)) " has been skilled up !") "NewEnumerator1")
      (return true))))

(fn GetCastingAbility
  (return 0))

(fn GetName
  (return (Variables|Attributes|GetAbilityName)))