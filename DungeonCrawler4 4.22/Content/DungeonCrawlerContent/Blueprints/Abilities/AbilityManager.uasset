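; Actor that manages a Dungeon Crawler character's abilities, spawning each class in the owner's list as an ability actor held in an indexed array.
; It applies cooldown reduction and attack speed to abilities, relays reset, interrupt and planning-stop calls, and finds abilities by class or casting state.
; It also tracks skill points with widget toggles, swaps slots while refreshing the player HUD, and destroys itself and its abilities on owner EndPlay.
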(event Custom|DCOwnerEndPlay
  (params (Actor :type Actor%20Object%20Reference) (EndPlayReason :type EEndPlayReason%20Enum :default "Destroyed"))
  (for _array_element (Variables|Default|GetAbilities)
    (Utilities|IsValid _array_element
      (:Is%20Valid
        (Actor|DestroyActor _array_element))))
  (Actor|DestroyActor))

(event EventBeginPlay
  (Game|AssignOnEndPlay (Variables|Default|GetDCOwner) (delegate Custom|DCOwnerEndPlay)))

(fn ConstructionScript)

(fn InitAbilities
  (for _array_element (Variables|Default|GetAbilities)
    (Utilities|IsValid _array_element
      (:Is%20Valid
        (Default|Init _array_element)))))

(fn Init
  (if (> (Utilities|Array|Length (Variables|Default|GetAbilities)) 1)
    _
    (else
      (for (_array_element _array_index) (Variables|/Game/DungeonCrawlerContent/Blueprints/Characters/DCBaseCharacter.DCBaseCharacter_C|GetAbilities (Variables|Default|GetDCOwner))
        (bind _ability (CallFunction|SetAbility _array_element _array_index))
        (Utilities|Array|AddUnique (Variables|Default|GetAbilities) _ability))))
  (CallFunction|InitAbilities))

(fn SetAbilityCooldowns
  (for _array_element (Variables|Default|GetAbilities)
    (Utilities|IsValid _array_element
      (:Is%20Valid
        (Default|SetCooldownfromPercentage _array_element (Utilities|Struct|BreakCharacterAttributes (Variables|/Game/DungeonCrawlerContent/Blueprints/Characters/DCBaseCharacter.DCBaseCharacter_C|GetAttributes (Variables|Default|GetDCOwner))))))))

(fn SetAbilityCastTimes
  (for _array_element (Variables|Default|GetAbilities)
    (bind _ascastable_ability (Utilities|Casting|CastToCastableAbility _array_element))
    (Default|SetCastTimefromPercentage _ascastable_ability (Utilities|Struct|BreakCharacterAttributes (Variables|/Game/DungeonCrawlerContent/Blueprints/Characters/DCBaseCharacter.DCBaseCharacter_C|GetAttributes (Variables|Default|GetDCOwner))))))

(fn ResetAbilities
  (for _array_element (Variables|Default|GetAbilities)
    (Default|Reset _array_element)))

(fn InteruptCastableAbilities
  (for _array_element (Variables|Default|GetAbilities)
    (Class|AbilityInterface|OnInteruptCasting(Message) _array_element)))

(fn GetCastingAbility
  (for _array_element (Variables|Default|GetAbilities)
    (bind _castingability (Class|AbilityInterface|GetCastingAbility(Message) _array_element))
    (Utilities|IsValid _castingability
      (:Is%20Valid
        (LocalVariables|SettempAbility _castingability))))
  (return (LocalVariables|GettempAbility)))

(fn ToggleSkillUpUI
  (params (On :type Boolean))
  (for _array_element (Variables|Default|GetAbilities)
    (Utilities|IsValid (Variables|/Game/DungeonCrawlerContent/Blueprints/Abilities/Ability.Ability_C|GetAbilityWidgetRef _array_element)
      (:Is%20Valid
        (Default|ToggleSkillUp (Variables|/Game/DungeonCrawlerContent/Blueprints/Abilities/Ability.Ability_C|GetAbilityWidgetRef _array_element) On)))))

(fn SkillUpAbility
  (params (Ability :type Ability%20Object%20Reference))
  (bind _skillpoints (Variables|Default|GetSkillPoints))
  (Default|SkillUp Ability)
  (Math|Integer|DecrementInt _skillpoints
    (:%20%20
      (if (<= _skillpoints 0)
        (CallFunction|ToggleSkillUpUI false)))))

(fn ReadySkillUp
  (Math|Integer|IncrementInt (Variables|Default|GetSkillPoints)
    (:%20%20
      (CallFunction|ToggleSkillUpUI true))))

(fn SetAbility
  (params (NewAbility :type Ability%20Class%20Reference) (Index :type Integer))
  (bind _returnvalue (Game|SpawnActorfromClass NewAbility (Math|Transform|MakeTransform "0, 0, 0") "Undefined" 0 (Variables|Default|GetDCOwner) self 0))
  (Utilities|Array|SetArrayElem (Variables|Default|GetAbilities) Index _returnvalue)
  (return _returnvalue))

(fn SwapAbility
  (params (Ability :type Ability%20Class%20Reference) (Slot :type Integer) (DestroyOld? :type Boolean))
  (bind _abilities (Variables|Default|GetAbilities))
  (bind _output (Utilities|Array|Get(acopy) _abilities Slot))
  (Utilities|IsValid _output
    (:Is%20Valid
      (bind _output_get (LocalVariables|SetTempAbility _output))
      (Default|Reset _output_get)
      (Utilities|Array|SetArrayElem (Variables|Default|GetAbilities) Slot 0)
      (if DestroyOld?
        (Actor|DestroyActor (LocalVariables|GetTempAbility))))
    (:Is%20Not%20Valid
      _))
  (bind _ability (CallFunction|SetAbility Ability Slot))
  (Default|Init _ability)
  (bind _asdcplayer_character (Utilities|Casting|CastToDCPlayerCharacter (Variables|Default|GetDCOwner)))
  (Default|CreateAbilityWidget (Variables|/Game/DungeonCrawlerContent/Blueprints/Controllers/DCPlayerController.DCPlayerController_C|GetDCHUD (Variables|/Game/DungeonCrawlerContent/Blueprints/Characters/PlayerCharacters/DCPlayerCharacter.DCPlayerCharacter_C|GetDCPlayerController _asdcplayer_character)) Slot))

(fn GetAbilityOfClass
  (params (AbilityClass :type Ability%20Class%20Reference))
  (bind _array_element (Utilities|Array|ForEachLoopwithBreak (Variables|Default|GetAbilities))
    (:LoopBody
      (if (== AbilityClass (Utilities|GetClass _array_element))
        (LocalVariables|SetMatchingAbility _array_element)))
    (:Completed
      (Utilities|IsValid (LocalVariables|GetMatchingAbility)
        (:Is%20Valid
          (return true (LocalVariables|GetMatchingAbility)))
        (:Is%20Not%20Valid
          (return false 0))))))

(fn StopPlanning
  (Variables|Default|SetIsPlanning false)
  (Utilities|IsValid (Variables|Default|GetPlanningAbility)
    (:Is%20Valid
      (Class|IPlanningAbility|AbilityPlanStop(Message) (Variables|Default|GetPlanningAbility))
      (Variables|Default|SetPlanningAbility 0))))