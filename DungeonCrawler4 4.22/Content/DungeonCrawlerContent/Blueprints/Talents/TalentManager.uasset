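; TalentManager is an actor that manages a character's tiered talent choices in the dungeon crawler.
; Init spawns an actor for each talent class in the owner's tier definitions, storing them by tier and unlock level.
; Level checks reveal matching UI rows; choosing a talent applies it, hides that row and sends a message.
; It can also apply all selected talents, and destroys them and itself when the owner ends play.
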(event Custom|DCOwnerEndPlay
  (params (Actor :type Actor%20Object%20Reference) (EndPlayReason :type EEndPlayReason%20Enum))
  (for _array_element (Variables|Default|GetTalents)
    (for _array_element_2 (Utilities|Struct|BreakTalentTier _array_element)
      (Actor|DestroyActor _array_element_2)))
  (Actor|DestroyActor))

(event EventBeginPlay
  (Game|AssignOnEndPlay (Variables|Default|GetDCOwner) (delegate Custom|DCOwnerEndPlay)))

(fn ConstructionScript)

(fn Init
  (for (_array_element _array_index) (Variables|/Game/DungeonCrawlerContent/Blueprints/Characters/DCBaseCharacter.DCBaseCharacter_C|GetTalents (Variables|Default|GetDCOwner))
    (for _array_element_2 (.TalentOptions (Utilities|Struct|BreakBaseTalentTier _array_element))
      ;[1 1 1] row
      (if (Utilities|IsValidClass _array_element_2)
        (LocalVariables|SettempToSpawn _array_element_2))
      (bind _returnvalue (Game|SpawnActorfromClass (LocalVariables|GettempToSpawn) (Math|Transform|MakeTransform "0, 0, 0") "Undefined" 0 (Variables|Default|GetDCOwner) self _array_index))
      (Utilities|Array|Add (LocalVariables|Gettemprow) _returnvalue))
    (Utilities|Array|Add (LocalVariables|GettempTalents) (Utilities|Struct|MakeTalentTier (LocalVariables|Gettemprow) (.ObtainableAt (Utilities|Struct|BreakBaseTalentTier _array_element))))
    (Utilities|Array|Clear (LocalVariables|Gettemprow)))
  (Variables|Default|SetTalents (LocalVariables|GettempTalents)))

(fn SetTalent
  (params (Talent :type Talent%20Object%20Reference))
  (bind _tier (Variables|/Game/DungeonCrawlerContent/Blueprints/Talents/Talent.Talent_C|GetTier Talent))
  (Default|ApplyTalent Talent)
  (CallFunction|SetRow false _tier)
  (Class|MessageInterface|SendMessage(Message) (Game|GetGameInstance) (Utilities|String|Append (Utilities|String|ToString(Name) (Variables|/Game/DungeonCrawlerContent/Blueprints/Characters/DCBaseCharacter.DCBaseCharacter_C|GetCharacterName (Variables|Default|GetDCOwner))) " has chosen " (Utilities|String|ToString(Name) (Variables|/Game/DungeonCrawlerContent/Blueprints/Talents/Talent.Talent_C|GetTalentName Talent)) " as their tier " (Utilities|String|ToString(Integer) _tier) " talent.") "NewEnumerator4"))

(fn SetRow
  (params (On :type Boolean) (Tier :type Integer))
  (bind _gameui (Variables|Default|GetGameUI))
  (Utilities|IsValid _gameui
    (:Is%20Valid
      (Default|ToggleTalentRow _gameui On Tier))))

(fn CheckTalentAvailable
  (params (LeveltoCheck :type Integer))
  (for (_array_element _array_index) (Variables|Default|GetTalents)
    (if (== LeveltoCheck (.ObtainableAt (Utilities|Struct|BreakTalentTier _array_element)))
      (CallFunction|SetRow true _array_index))))

(fn ApplySelectedTalents
  (for _array_element (Variables|Default|GetTalents)
    (for _array_element_2 (Utilities|Struct|BreakTalentTier _array_element)
      (if (Variables|/Game/DungeonCrawlerContent/Blueprints/Talents/Talent.Talent_C|GetSelected _array_element_2)
        (Default|ApplyTalent _array_element_2)))))