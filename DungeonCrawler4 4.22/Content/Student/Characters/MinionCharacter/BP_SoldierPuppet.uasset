(event EventUseTakeYourPositions
  (params (TargetLocation :type Vector :default "0, 0, 0"))
  (bind _abilitymanager (Variables|Default|GetAbilityManager))
  (bind _abilities (Variables|/Game/DungeonCrawlerContent/Blueprints/Abilities/AbilityManager.AbilityManager_C|GetAbilities _abilitymanager))
  (bind _output (Utilities|Array|Get(acopy) _abilities 3))
  (Class|IAbilityVariableSetters|SetTargetLocation(Message) _output TargetLocation)
  (Default|ExecuteAbility _output))

(event EventModifyExperience
  (params (Amount :type Integer) (Positive :type Boolean))
  ;[1 1 1] Override so it dosn't do anything
)

(event EventUsefortheLegion
  (Default|ExecuteAbility (Utilities|Array|Get(acopy) (Variables|/Game/DungeonCrawlerContent/Blueprints/Abilities/AbilityManager.AbilityManager_C|GetAbilities (Variables|Default|GetAbilityManager)) 4)))

(event EventUseWeStrikeasOne
  (params (TargetEnemy :type DC%20Base%20Character%20Object%20Reference))
  (bind _abilitymanager (Variables|Default|GetAbilityManager))
  (bind _abilities (Variables|/Game/DungeonCrawlerContent/Blueprints/Abilities/AbilityManager.AbilityManager_C|GetAbilities _abilitymanager))
  (bind _output (Utilities|Array|Get(acopy) _abilities 2))
  (Variables|/Game/DungeonCrawlerContent/Blueprints/Abilities/Ability.Ability_C|SetTarget _output TargetEnemy)
  (Default|ExecuteAbility _output))

(fn ConstructionScript
  (|CallParentFunction))

(fn Death
  (bind _success (|CallParentFunction))
  (Class|IMinionManagment|MinionHasDied(Message) (Variables|Default|GetLeader) self)
  (Actor|DestroyActor)
  (return _success))

(fn Init
  (params (Level :type Integer) (Team :type Integer))
  (bind _success (|CallParentFunction Level Team))
  (EventDispatchers|BindEventtoOnKill (EventDispatchers|CreateEvent :!event PassKilltoLeader))
  (return _success))

(fn PassKilltoLeader
  (params (ID :type DC%20Base%20Character%20Object%20Reference)))