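; BP_PuppetMaster is a player character class that commands minions and holds state for its Master's Mark ability.
; It adds and removes minion references through events, and LevelUp runs the parent logic, then levels every tracked minion.
; The construction script gathers four minion spawn locations, exposed through a getter alongside the minion list.
; Setters and getters expose whether Master's Mark can apply damage over time or crit, plus its stack count.
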(event EventAddMinionRef
  (params (NewMinion :type Companion%20Character%20Object%20Reference))
  (Utilities|Array|AddUnique (Variables|Default|GetMinions) NewMinion))

(event EventMinionHasDied
  (params (MinionWhoDied :type Companion%20Character%20Object%20Reference))
  (Utilities|Array|RemoveItem (Variables|Default|GetMinions) MinionWhoDied))

(event EventSetMastersMarkDOT
  (params (On :type Boolean))
  (Variables|MastersMark|SetMastersMarkCanApplyDOT On))

(event EventSetMastersMarkCritChange
  (params (On :type Boolean))
  (Variables|MastersMark|SetMastersMarkCanApplyCrit On))

(event EventSetMastersMarkStackCount
  (params (Count :type Integer))
  (Variables|MastersMark|SetMastersMarkStackCount Count))

(fn ConstructionScript
  (bind _minionspawnlocations (Variables|Default|GetMinionSpawnLocations))
  (|CallParentFunction)
  (Utilities|Array|AddUnique _minionspawnlocations (Variables|Default|GetMinionLocation1))
  (Utilities|Array|AddUnique _minionspawnlocations (Variables|Default|GetMinionLocation2))
  (Utilities|Array|AddUnique _minionspawnlocations (Variables|Default|GetMinionLocation3))
  (Utilities|Array|AddUnique _minionspawnlocations (Variables|Default|GetMinionLocation4)))

(fn Init
  (params (Level :type Integer) (Team :type Integer))
  (bind _success (|CallParentFunction Level Team))
  (return _success))

(fn LevelUp
  (bind _success (|CallParentFunction))
  (for _array_element (Variables|Default|GetMinions)
    (CallFunction|LevelUp _array_element))
  (return _success))

(fn GetAllMinions
  (return (Variables|Default|GetMinions)))

(fn GetAllSpawnLocations
  (return (Variables|Default|GetMinionSpawnLocations)))

(fn GetMastersMarkCritChange
  (return (Variables|MastersMark|GetMastersMarkCanApplyCrit)))

(fn GetMastersMarkDOT
  (return (Variables|MastersMark|GetMastersMarkCanApplyDOT)))

(fn GetMastersMarkStackCount
  (return (Variables|MastersMark|GetMastersMarkStackCount)))